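; BP_InteractableParticles is an interactable Blueprint that shows an interaction prompt while the player is nearby.
; On BeginPlay it passes its InteractionText to the W_InteractionPrompt hosted in its Widget component.
; InteractionZone overlaps filtered to MyCharacter toggle the widget's visibility and the PlayerInZone flag.
; Despite the name, its graphs contain no particle logic or handling of the interaction itself.
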(event OnComponentBeginOverlap(InteractionZone)
  (params (OverlappedComponent :type Primitive%20Component%20Object%20Reference) (OtherActor :type Actor%20Object%20Reference) (OtherComp :type Primitive%20Component%20Object%20Reference) (OtherBodyIndex :type Integer) (bFromSweep :type Boolean) (SweepResult :type Hit%20Result%20Structure%20%28by%20ref%29))
  ;[1 0.1979 0.1979] Controlar Visualización de WIDGET DE INTERACCIÓN
  ;;[1 1 1] Mostrar el Widget cuando el jugador entra al Area de interaccion
  ;;;[1 1 1] Casteamos el Actor Solapado como el Player
  (Utilities|Casting|CastToMyCharacter OtherActor)
  ;;;[1 1 1] Activamos el Flag de Jugador en Zona
  (Variables|Default|SetPlayerInZone true)
  (Rendering|SetVisibility (Variables|Default|GetWidget) true false))

(event OnComponentEndOverlap(InteractionZone)
  (params (OverlappedComponent :type Primitive%20Component%20Object%20Reference) (OtherActor :type Actor%20Object%20Reference) (OtherComp :type Primitive%20Component%20Object%20Reference) (OtherBodyIndex :type Integer))
  ;[1 0.1979 0.1979] Controlar Visualización de WIDGET DE INTERACCIÓN
  ;;[1 1 1] Ocultar el Widget cuando el jugador sale del Area de interaccion
  ;;;[1 1 1] Casteamos el Actor Solapado como el Player
  (Utilities|Casting|CastToMyCharacter OtherActor)
  ;;;[1 1 1] Desactivamos el Flag de Jugador en Zona
  (Variables|Default|SetPlayerInZone false)
  (Rendering|SetVisibility (Variables|Default|GetWidget) false false))

(event EventBeginPlay
  ;[1 0.2289 0.2488] Asignar Texto de Interacción al Widget
  ;;[1 1 1] Obtenemos el tipo de Widget usado para este componente, y lo casteamos como Prompt de Interacción
  (bind _asw_interaction_prompt (Utilities|Casting|CastToW_InteractionPrompt (UserInterface|GetWidget (Variables|Default|GetWidget))))
  ;;[1 1 1] Seteamos el Texto que aparecerá en el Prompt de Interaccion
  (Default|SetInteractionText _asw_interaction_prompt (Variables|Default|GetInteractionText)))

(fn ConstructionScript)