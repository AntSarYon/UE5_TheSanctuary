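; BP_Pickeable is an interactable object the player can pick up and carry, with a widget that is hidden while it is held.
; Each Tick it casts the player pawn to MyCharacter and hides the Widget if IsGrabbingObject is set and GrabbedObject is this actor.
; This graph only hides the widget and never shows it again; the grab logic itself is not in this file.
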(event EventBeginPlay
  (|CallParentFunction) ; This node is disabled and will not be called.\nDrag off pins to build functionality.
)

(event Collision|EventActorBeginOverlap
  (params (OtherActor :type Actor%20Object%20Reference)))

(event EventTick
  (params (DeltaSeconds :type Float%20%28single-precision%29))
  ;[1 0.4628 0.403] Controlar Visualización de Widget, cuando el Jugador esta cargando el Objeto
  ;;[0.08854 0.08739 0.08648] Revisamos si el jugador esta cargando un objeto, y si ese objeto somos nosotros
  (bind _asmy_character (Utilities|Casting|CastToMyCharacter (Game|Player|GetPlayerPawn 0)))
  (if (and (Variables|/Game/MyBlueprints/MyCharacter.MyCharacter_C|GetisGrabbingObject _asmy_character) (== (Variables|/Game/MyBlueprints/MyCharacter.MyCharacter_C|GetGrabbedObject _asmy_character) self))
    ;;[1 1 1] Si es el caso, Ocultamos el Widget
    (Rendering|SetVisibility (Variables|Default|GetWidget) false false)))

(fn ConstructionScript
  (|CallParentFunction))